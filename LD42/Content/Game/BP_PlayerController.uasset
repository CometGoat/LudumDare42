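; Player controller for a mouse-driven puzzle of placing modules, tied to the brain actor and mission texts.
; Startup sets the camera and text widget, spawns four modules and presents the briefing.
; Each module gets a random connected four-cell shape on a 3x3 grid, grown by retrying picks, plus an unused mission string.
; Cursor traces drag unlocked modules and attempt locking on release; choose mode instead sends the clicked module's string to BP_AllTexts.
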(event Custom|ChooseModule
  (Variables|Default|SetChoosingModule true))

(event Custom|PieceChosen
  (params (BP_Module :type BP%20Module%20Object%20Reference))
  (Variables|Default|SetChoosingModule false)
  (bind _outactors (Actor|GetAllActorsOfClass "/Game/Blueprints/BP_AllTexts.BP_AllTexts_C"))
  (Default|CalculateChoice (Utilities|Array|Get(acopy) _outactors) (Variables|/Game/Blueprints/BP_Module.BP_Module_C|GetModuleString BP_Module)))

(event Custom|SpawnModules
  (bind _currentmission (Variables|Default|GetCurrentMission))
  (bind _bp_alltexts (Variables|Default|GetBP_AllTexts))
  (bind _pattern (Variables|Default|GetPattern))
  (bind _pattern_2 (Variables|Default|GetPattern))
  (bind _modulespacing (Variables|Default|GetModuleSpacing))
  (bind _pattern_3 (Variables|Default|GetPattern))
  (bind _returnvalue (Utilities|Array|LastIndex _pattern))
  (bind _returnvalue_2 (* _modulespacing 2.0))
  (bind _mission_1_1 (Variables|/Game/Blueprints/BP_AllTexts.BP_AllTexts_C|GetMission_1_1 _bp_alltexts))
  (bind _returnvalue_3 (Math|Random|RandomIntegerinRange 0 _returnvalue))
  (bind _returnvalue_4 (Utilities|Select :Index _currentmission :Option%200 _mission_1_1 :Option%201 ""))
  (Utilities|Array|Clear (Variables|Default|GetCurrentStrings))
  (for _index (range 0 3)
    (Utilities|Array|Clear _pattern_3)
    (Utilities|Array|Resize _pattern_3 9)
    (Utilities|Array|SetArrayElem _pattern _returnvalue_3 1)
    (for _index_2 (range 0 2)
      (Variables|Default|SetPieceAccepted false)
      (Variables|Default|SetSuggestedPiece _returnvalue_3 :!label _label)
      (Variables|Default|SetAcceptedModulo false)
      (Variables|Default|SetAcceptedDivision false)
      (if (== (Utilities|Array|Get(acopy) _pattern_2 (Variables|Default|GetSuggestedPiece)) 0)
        (for (_array_element _array_index) _pattern_2
          (if (== _array_element 1)
            (if (and (== (Math|Integer|%(Integer) (Variables|Default|GetSuggestedPiece) 3) (Math|Integer|%(Integer) _array_index 3)) (or (== (- (/ _array_index 3) (/ (Variables|Default|GetSuggestedPiece) 3)) 1) (== (- (/ _array_index 3) (/ (Variables|Default|GetSuggestedPiece) 3)) -1)))
              (Variables|Default|SetPieceAccepted true)
              (elif (and (== (/ (Variables|Default|GetSuggestedPiece) 3) (/ _array_index 3)) (or (== (- (Math|Integer|%(Integer) _array_index 3) (Math|Integer|%(Integer) (Variables|Default|GetSuggestedPiece) 3)) 1) (== (- (Math|Integer|%(Integer) _array_index 3) (Math|Integer|%(Integer) (Variables|Default|GetSuggestedPiece) 3)) -1)))
                (Variables|Default|SetPieceAccepted true)))))
        (if (Variables|Default|GetPieceAccepted)
          (Utilities|Array|SetArrayElem (Variables|Default|GetPattern) (Variables|Default|GetSuggestedPiece) 1)
          (else
            (goto _label)))
        (else
          (goto _label))))
    (Development|PrintString "Generation complete!")
    (bind _output_get (Variables|Default|SetSuggestedString (Utilities|Array|Get(acopy) (.modules _returnvalue_4) (Math|Random|RandomIntegerinRange 0 (Utilities|Array|LastIndex (.modules _returnvalue_4)))) :!label _label_2))
    (if (or (Utilities|Array|ContainsItem (Variables|/Game/Blueprints/BP_Brain.BP_Brain_C|GetInstalledModules (Variables|Default|GetBP_Brain)) (Variables|Default|GetSuggestedString)) (Utilities|Array|ContainsItem (Variables|Default|GetCurrentStrings) (Variables|Default|GetSuggestedString)))
      (goto _label_2)
      (else
        (Utilities|Array|Add (Variables|Default|GetCurrentStrings) _output_get)
        (Game|SpawnActorfromClass "/Game/Blueprints/BP_Module.BP_Module_C" (Math|Transform|MakeTransform (+ (- (Math|Vector|MakeVector (* (/ (+ (Math|Integer|%(Integer) _index 2) 1) 2) _modulespacing) (* (/ (+ (/ _index 2) 1) 2) _modulespacing) 2e+02) (Math|Vector|MakeVector _returnvalue_2 _returnvalue_2 0.0)) "2500.000000,4100.000000, 0") "0,-90.000000, 0" "1.000000,1.000000,1.000000") "AlwaysSpawn" 0 (Variables|Default|GetPattern) (Variables|Default|GetSuggestedString) 0)))))

(event Custom|CalculatePattern
  (bind _currentmission (Variables|Default|GetCurrentMission))
  (bind _bp_alltexts (Variables|Default|GetBP_AllTexts))
  (bind _pattern (Variables|Default|GetPattern))
  (bind _pattern_2 (Variables|Default|GetPattern))
  (bind _modulespacing (Variables|Default|GetModuleSpacing))
  (bind _returnvalue (Utilities|Array|LastIndex _pattern))
  (bind _returnvalue_2 (* _modulespacing 2.0))
  (bind _mission_1_1 (Variables|/Game/Blueprints/BP_AllTexts.BP_AllTexts_C|GetMission_1_1 _bp_alltexts))
  (bind _returnvalue_3 (Math|Random|RandomIntegerinRange 0 _returnvalue))
  (bind _returnvalue_4 (Utilities|Select :Index _currentmission :Option%200 _mission_1_1 :Option%201 ""))
  (Utilities|Array|SetArrayElem _pattern _returnvalue_3 1)
  (for _index (range 0 2)
    (Variables|Default|SetPieceAccepted false)
    (Variables|Default|SetSuggestedPiece _returnvalue_3 :!label _label)
    (Variables|Default|SetAcceptedModulo false)
    (Variables|Default|SetAcceptedDivision false)
    (if (== (Utilities|Array|Get(acopy) _pattern_2 (Variables|Default|GetSuggestedPiece)) 0)
      (for (_array_element _array_index) _pattern_2
        (if (== _array_element 1)
          (if (and (== (Math|Integer|%(Integer) (Variables|Default|GetSuggestedPiece) 3) (Math|Integer|%(Integer) _array_index 3)) (or (== (- (/ _array_index 3) (/ (Variables|Default|GetSuggestedPiece) 3)) 1) (== (- (/ _array_index 3) (/ (Variables|Default|GetSuggestedPiece) 3)) -1)))
            (Variables|Default|SetPieceAccepted true)
            (elif (and (== (/ (Variables|Default|GetSuggestedPiece) 3) (/ _array_index 3)) (or (== (- (Math|Integer|%(Integer) _array_index 3) (Math|Integer|%(Integer) (Variables|Default|GetSuggestedPiece) 3)) 1) (== (- (Math|Integer|%(Integer) _array_index 3) (Math|Integer|%(Integer) (Variables|Default|GetSuggestedPiece) 3)) -1)))
              (Variables|Default|SetPieceAccepted true)))))
      (if (Variables|Default|GetPieceAccepted)
        (Utilities|Array|SetArrayElem (Variables|Default|GetPattern) (Variables|Default|GetSuggestedPiece) 1)
        (else
          (goto _label)))
      (else
        (goto _label))))
  (Development|PrintString "Generation complete!")
  (bind _output_get (Variables|Default|SetSuggestedString (Utilities|Array|Get(acopy) (.modules _returnvalue_4) (Math|Random|RandomIntegerinRange 0 (Utilities|Array|LastIndex (.modules _returnvalue_4)))) :!label _label_2))
  (if (or (Utilities|Array|ContainsItem (Variables|/Game/Blueprints/BP_Brain.BP_Brain_C|GetInstalledModules (Variables|Default|GetBP_Brain)) (Variables|Default|GetSuggestedString)) (Utilities|Array|ContainsItem (Variables|Default|GetCurrentStrings) (Variables|Default|GetSuggestedString)))
    (goto _label_2)
    (else
      (Utilities|Array|Add (Variables|Default|GetCurrentStrings) _output_get)
      (Game|SpawnActorfromClass "/Game/Blueprints/BP_Module.BP_Module_C" (Math|Transform|MakeTransform (+ (- (Math|Vector|MakeVector (* (/ (+ (Math|Integer|%(Integer) (stale Custom|SpawnModules _index) 2) 1) 2) _modulespacing) (* (/ (+ (/ (stale Custom|SpawnModules _index) 2) 1) 2) _modulespacing) 2e+02) (Math|Vector|MakeVector _returnvalue_2 _returnvalue_2 0.0)) "2500.000000,4100.000000, 0") "0,-90.000000, 0" "1.000000,1.000000,1.000000") "AlwaysSpawn" 0 (Variables|Default|GetPattern) (Variables|Default|GetSuggestedString) 0))))

(event Custom|SpawnMoreModules
  (bind _outactors (Actor|GetAllActorsOfClass "/Game/Blueprints/BP_Module.BP_Module_C"))
  (for _array_element _outactors
    (if (not (Variables|/Game/Blueprints/BP_Module.BP_Module_C|GetLocked _array_element))
      (Actor|DestroyActor _array_element)))
  (CallFunction|SpawnModules))

(event Custom|ResetModuleLockButtonSet
  (Utilities|FlowControl|DoOnce false) ; enters at Reset
)

(event Custom|PresentBriefing
  (params (Mission :type Integer))
  (Default|MissionBriefing (Variables|Default|GetBP_AllTexts) Mission))

(event EventBeginPlay
  (bind _returnvalue (UserInterface|CreateWidget "/Game/UI/Widgets/W_TextBox.W_TextBox_C"))
  (UserInterface|Viewport|AddtoViewport _returnvalue 0)
  (Variables|Default|SetW_TextBox _returnvalue)
  (bind _outactors (Actor|GetAllActorsOfClass "/Game/Blueprints/BP_Brain.BP_Brain_C"))
  (Variables|Default|SetBP_Brain (Utilities|Array|Get(acopy) _outactors))
  (bind _outactors_2 (Actor|GetAllActorsOfClass "/Game/Blueprints/BP_Camera.BP_Camera_C"))
  (Game|Player|SetViewTargetwithBlend (Utilities|Array|Get(acopy) _outactors_2) 0.0 "VTBlend_Linear" 0.0 false)
  (Variables|Default|SetBP_Camera (Utilities|Array|Get(acopy) _outactors_2))
  (Variables|Default|SetbShowMouseCursor true)
  (bind _outactors_3 (Actor|GetAllActorsOfClass "/Game/Blueprints/BP_AllTexts.BP_AllTexts_C"))
  (Variables|Default|SetBP_AllTexts (Utilities|Array|Get(acopy) _outactors_3))
  (CallFunction|SpawnModules)
  (Variables|/Game/Blueprints/BP_AllTexts.BP_AllTexts_C|SetW_TextBox (Variables|Default|GetBP_AllTexts) (Variables|Default|GetW_TextBox))
  (CallFunction|PresentBriefing))

(event EventTick
  (params (DeltaSeconds :type Float%20%28single-precision%29))
  (bind (_hitresult _returnvalue) (Game|Player|GetHitResultUnderCursorbyChannel "TraceTypeQuery2" true))
  (bind _selectedmodule (Variables|Default|GetSelectedModule))
  (bind _moveoffset (Variables|Default|GetMoveOffset))
  (bind (_bblockinghit _binitialoverlap _time _distance _location _impactpoint _normal _impactnormal _physmat _hitactor) (Collision|BreakHitResult _hitresult))
  (bind _returnvalue_2 (+ _location _moveoffset))
  (Utilities|IsValid _selectedmodule
    (:Is%20Valid
      (if _returnvalue
        (Utilities|Casting|CastToBP_Module _hitactor
          (:CastFailed
            (Transformation|SetActorLocation _selectedmodule (Math|Vector|MakeVector (.x _returnvalue_2) (.y _returnvalue_2) 2e+02) false false)
            (Default|IftheShoeFits (Variables|Default|GetSelectedModule))))))))

(event Input|MouseEvents|LeftMouseButton
  (params (Key :type Key%20Structure))
  (bind (_hitresult _returnvalue) (Game|Player|GetHitResultUnderCursorbyChannel "TraceTypeQuery1" true))
  (:Pressed
    (if _returnvalue
      (bind _asbp_module_piece (Utilities|Casting|CastToBP_ModulePiece (.HitActor (Collision|BreakHitResult _hitresult))))
      (Development|PrintString "Dat a module")
      (if (Variables|Default|GetChoosingModule)
        (CallFunction|PieceChosen (.AsBP%20Module (Utilities|Casting|CastToBP_Module (Actor|GetParentActor _asbp_module_piece))))
        (Development|PrintString "Piece chosen!")
        (elif (not (Variables|/Game/Blueprints/BP_Module.BP_Module_C|GetLocked (.AsBP%20Module (Utilities|Casting|CastToBP_Module (Actor|GetParentActor _asbp_module_piece)))))
          (Variables|Default|SetSelectedModule (.AsBP%20Module (Utilities|Casting|CastToBP_Module (Actor|GetParentActor _asbp_module_piece))))
          (Variables|Default|SetMoveOffset (Math|Vector|MakeVector (.x (- (Transformation|GetActorLocation (Variables|Default|GetSelectedModule)) (.Location (Collision|BreakHitResult (.HitResult (Game|Player|GetHitResultUnderCursorbyChannel "TraceTypeQuery2" true)))))) (.y (- (Transformation|GetActorLocation (Variables|Default|GetSelectedModule)) (.Location (Collision|BreakHitResult (.HitResult (Game|Player|GetHitResultUnderCursorbyChannel "TraceTypeQuery2" true)))))) 0.0))))))
  (:Released
    (Utilities|IsValid (Variables|Default|GetSelectedModule)
      (:Is%20Valid
        (Default|LockModule (Variables|Default|GetSelectedModule))
        (if (Variables|/Game/Blueprints/BP_Module.BP_Module_C|GetLocked (Variables|Default|GetSelectedModule))
          (Utilities|FlowControl|Sequence
            (:then_0
              (Utilities|FlowControl|DoOnce false
                (:Completed
                  (Default|BindStart (Variables|Default|GetW_TextBox)))))
            (:then_1
              _)))
        (Variables|Default|SetSelectedModule 0)))))

(fn ConstructionScript)