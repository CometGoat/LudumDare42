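; BP_Module is a multi-cell puzzle piece that installs onto BP_Tile actors as a named module.
; The construction script spawns BP_ModulePiece child actors from the Shape grid and fits the name label along its densest row or column.
; IfTheShoeFits line-traces down from each piece to preview validity.
; LockModule re-traces, then either snaps, registers with BP_Brain and requests new modules, or resets position; used/refresh events toggle its tint.
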(event Custom|IfTheShoeFits
  (bind _invalidtiles (Variables|Default|GetInvalidTiles))
  (if (not (Variables|Default|GetAttemptingLock))
    (Variables|Default|SetAcceptedLocation true)
    (Utilities|Array|Clear (Variables|Default|GetInvalidTiles))
    (Utilities|Array|Clear (Variables|Default|GetValidTiles))
    (for _array_element (Variables|Default|GetPieces)
      (bind (_outhit _returnvalue) (Collision|LineTraceByChannel (Transformation|GetActorLocation _array_element) (+ (Transformation|GetActorLocation _array_element) "0, 0,-500.000000") "TraceTypeQuery2" false 0 "None"))
      (if _returnvalue
        (bind _asbp_tile (Utilities|Casting|CastToBP_Tile (.HitActor (Collision|BreakHitResult _outhit)))
          (:then
            (Utilities|IsValid (Variables|/Game/Blueprints/BP_Tile.BP_Tile_C|GetLockedPiece _asbp_tile)
              (:Is%20Valid
                (Variables|Default|SetAcceptedLocation false))
              (:Is%20Not%20Valid
                (Utilities|IsValid (Variables|/Game/Blueprints/BP_Tile.BP_Tile_C|GetSuggestedPiece _asbp_tile)
                  (:Is%20Valid
                    (Variables|Default|SetAcceptedLocation false :!label _label)
                    (Utilities|IsValid (Variables|/Game/Blueprints/BP_ModulePiece.BP_ModulePiece_C|GetTargettedTile _array_element)
                      (:Is%20Valid
                        (Rendering|Material|SetScalarParameterValueonMaterials (Variables|/Game/Blueprints/BP_Tile.BP_Tile_C|GetCube (Variables|/Game/Blueprints/BP_ModulePiece.BP_ModulePiece_C|GetTargettedTile _array_element)) "HueShift" 0.0)
                        (Variables|/Game/Blueprints/BP_ModulePiece.BP_ModulePiece_C|SetTargettedTile _array_element 0))))
                  (:Is%20Not%20Valid
                    (if (not (== (Variables|/Game/Blueprints/BP_ModulePiece.BP_ModulePiece_C|GetTargettedTile _array_element) _asbp_tile))
                      (Utilities|IsValid (Variables|/Game/Blueprints/BP_ModulePiece.BP_ModulePiece_C|GetTargettedTile _array_element)
                        (:Is%20Valid
                          (Utilities|Array|Add (Variables|Default|GetInvalidTiles) (Variables|/Game/Blueprints/BP_ModulePiece.BP_ModulePiece_C|GetTargettedTile _array_element)))
                        (:Is%20Not%20Valid
                          _))
                      (bind _output_get (Variables|/Game/Blueprints/BP_ModulePiece.BP_ModulePiece_C|SetTargettedTile _array_element _asbp_tile))
                      (Utilities|Array|Add (Variables|Default|GetValidTiles) _asbp_tile)
                      (Rendering|Material|SetScalarParameterValueonMaterials (Variables|/Game/Blueprints/BP_Tile.BP_Tile_C|GetCube _asbp_tile) "HueShift" 0.5)
                      (if (Utilities|Array|ContainsItem _invalidtiles _output_get)
                        (Utilities|Array|RemoveItem _invalidtiles _output_get))))))))
          (:CastFailed
            (goto _label)))
        (else
          (goto _label))))
    (for _array_element_2 (Variables|Default|GetInvalidTiles)
      (if (not (Utilities|Array|ContainsItem (Variables|Default|GetValidTiles) _array_element_2))
        (Rendering|Material|SetScalarParameterValueonMaterials (Variables|/Game/Blueprints/BP_Tile.BP_Tile_C|GetCube _array_element_2) "HueShift" 0.0)))
    (for _array_element_3 (Variables|Default|GetPieces)
      (Rendering|Material|SetMaterial (Variables|/Game/Blueprints/BP_ModulePiece.BP_ModulePiece_C|GetCube _array_element_3) 0 (select (Variables|Default|GetAcceptedLocation) "/Engine/EngineDebugMaterials/VertexColorViewMode_GreenOnly.VertexColorViewMode_GreenOnly" "/Engine/EngineDebugMaterials/VertexColorViewMode_RedOnly.VertexColorViewMode_RedOnly")))))

(event Custom|LockModule
  (bind _invalidtiles (Variables|Default|GetInvalidTiles))
  (bind _pieces (Variables|Default|GetPieces))
  (bind _modulestring (Variables|Default|GetModuleString))
  (bind _output (Utilities|Array|Get(acopy) _pieces))
  (bind _returnvalue (Actor|GetParentActor _output))
  (Variables|Default|SetAttemptingLock true)
  (Variables|Default|SetAcceptedLocation true)
  (Utilities|Array|Clear (Variables|Default|GetInvalidTiles))
  (Utilities|Array|Clear (Variables|Default|GetValidTiles))
  (for _array_element (Variables|Default|GetPieces)
    (bind (_outhit _returnvalue_2) (Collision|LineTraceByChannel (Transformation|GetActorLocation _array_element) (+ (Transformation|GetActorLocation _array_element) "0, 0,-500.000000") "TraceTypeQuery2" false 0 "None"))
    (if _returnvalue_2
      (bind _asbp_tile (Utilities|Casting|CastToBP_Tile (.HitActor (Collision|BreakHitResult _outhit)))
        (:then
          (Utilities|IsValid (Variables|/Game/Blueprints/BP_Tile.BP_Tile_C|GetLockedPiece _asbp_tile)
            (:Is%20Valid
              (Variables|Default|SetAcceptedLocation false))
            (:Is%20Not%20Valid
              (Utilities|IsValid (Variables|/Game/Blueprints/BP_Tile.BP_Tile_C|GetSuggestedPiece _asbp_tile)
                (:Is%20Valid
                  (Variables|Default|SetAcceptedLocation false :!label _label)
                  (Utilities|IsValid (Variables|/Game/Blueprints/BP_ModulePiece.BP_ModulePiece_C|GetTargettedTile _array_element)
                    (:Is%20Valid
                      (Rendering|Material|SetScalarParameterValueonMaterials (Variables|/Game/Blueprints/BP_Tile.BP_Tile_C|GetCube (Variables|/Game/Blueprints/BP_ModulePiece.BP_ModulePiece_C|GetTargettedTile _array_element)) "HueShift" 0.0)
                      (Variables|/Game/Blueprints/BP_ModulePiece.BP_ModulePiece_C|SetTargettedTile _array_element 0))))
                (:Is%20Not%20Valid
                  (if (== (Variables|/Game/Blueprints/BP_ModulePiece.BP_ModulePiece_C|GetTargettedTile _array_element) _asbp_tile)
                    (Utilities|Array|Add (Variables|Default|GetValidTiles) _asbp_tile)
                    (else
                      (Utilities|IsValid (Variables|/Game/Blueprints/BP_ModulePiece.BP_ModulePiece_C|GetTargettedTile _array_element)
                        (:Is%20Valid
                          (Utilities|Array|Add (Variables|Default|GetInvalidTiles) (Variables|/Game/Blueprints/BP_ModulePiece.BP_ModulePiece_C|GetTargettedTile _array_element)))
                        (:Is%20Not%20Valid
                          _))
                      (bind _output_get (Variables|/Game/Blueprints/BP_ModulePiece.BP_ModulePiece_C|SetTargettedTile _array_element _asbp_tile))
                      (Utilities|Array|Add (Variables|Default|GetValidTiles) _asbp_tile)
                      (Rendering|Material|SetScalarParameterValueonMaterials (Variables|/Game/Blueprints/BP_Tile.BP_Tile_C|GetCube _asbp_tile) "HueShift" 0.5)
                      (if (Utilities|Array|ContainsItem _invalidtiles _output_get)
                        (Utilities|Array|RemoveItem _invalidtiles _output_get)))))))))
        (:CastFailed
          (goto _label)))
      (else
        (goto _label))))
  (for _array_element_2 (Variables|Default|GetInvalidTiles)
    (if (not (Utilities|Array|ContainsItem (Variables|Default|GetValidTiles) _array_element_2))
      (Rendering|Material|SetScalarParameterValueonMaterials (Variables|/Game/Blueprints/BP_Tile.BP_Tile_C|GetCube _array_element_2) "HueShift" 0.0)))
  (for _array_element_3 (Variables|Default|GetPieces)
    _)
  (if (Variables|Default|GetAcceptedLocation)
    (for _array_element_4 _pieces
      (Variables|/Game/Blueprints/BP_Tile.BP_Tile_C|SetLockedPiece (Variables|/Game/Blueprints/BP_ModulePiece.BP_ModulePiece_C|GetTargettedTile _array_element_4) _array_element_4))
    (Transformation|SetActorLocation _returnvalue (+ (Transformation|GetActorLocation _returnvalue) (Math|Vector|MakeVector (.x (- (Transformation|GetActorLocation (Variables|/Game/Blueprints/BP_ModulePiece.BP_ModulePiece_C|GetTargettedTile _output)) (Transformation|GetActorLocation _output))) (.y (- (Transformation|GetActorLocation (Variables|/Game/Blueprints/BP_ModulePiece.BP_ModulePiece_C|GetTargettedTile _output)) (Transformation|GetActorLocation _output))) 0.0)) false false)
    (Variables|Default|SetLocked true)
    (bind _outactors (Actor|GetAllActorsOfClass "/Game/Blueprints/BP_Brain.BP_Brain_C"))
    (Utilities|Array|Add (Variables|/Game/Blueprints/BP_Brain.BP_Brain_C|GetInstalledModules (Utilities|Array|Get(acopy) _outactors)) _modulestring)
    (Development|PrintString (Utilities|String|Append "Installed " _modulestring " module"))
    (Default|SpawnMoreModules (.AsBP%20Player%20Controller (Utilities|Casting|CastToBP_PlayerController (Game|GetPlayerController 0))))
    (Utilities|FlowControl|Delay (Utilities|Time|GetWorldDeltaSeconds))
    (for _array_element_5 (Actor|GetAllChildActors true)
      (bind _asbp_module_piece (Utilities|Casting|CastToBP_ModulePiece _array_element_5))
      (Rendering|Material|SetMaterial (Variables|/Game/Blueprints/BP_ModulePiece.BP_ModulePiece_C|GetCube _asbp_module_piece) 0 "/Game/Material/M_Locked_Inst.M_Locked_Inst")
      (Rendering|Material|SetScalarParameterValueonMaterials (Variables|/Game/Blueprints/BP_ModulePiece.BP_ModulePiece_C|GetCube _asbp_module_piece) "HueShift" (Variables|Default|GetRandomHueShift))
      (Rendering|Material|SetScalarParameterValueonMaterials (Variables|/Game/Blueprints/BP_ModulePiece.BP_ModulePiece_C|GetCube _asbp_module_piece) "Desaturate" (Variables|Default|GetRandomSaturationShift)))
    (else
      (for _array_element_6 (Variables|Default|GetValidTiles)
        (Rendering|Material|SetScalarParameterValueonMaterials (Variables|/Game/Blueprints/BP_Tile.BP_Tile_C|GetCube _array_element_6) "HueShift" 0.0))
      (Variables|Default|SetAttemptingLock false)
      (Transformation|SetActorLocation (Variables|Default|GetStartPosition) false false)
      (for _array_element_7 (Variables|Default|GetPieces)
        (Rendering|Material|SetMaterial (Variables|/Game/Blueprints/BP_ModulePiece.BP_ModulePiece_C|GetCube _array_element_7) 0 "/Engine/EngineMaterials/DefaultDecalMaterial.DefaultDecalMaterial"))
      (CallFunction|ColourChange))))

(event Custom|ColourChange
  (for _array_element (Actor|GetAllChildActors true)
    (bind _asbp_module_piece (Utilities|Casting|CastToBP_ModulePiece _array_element))
    (Rendering|Material|SetMaterial (Variables|/Game/Blueprints/BP_ModulePiece.BP_ModulePiece_C|GetCube _asbp_module_piece) 0 "/Game/Material/M_Locked_Inst.M_Locked_Inst")
    (Rendering|Material|SetScalarParameterValueonMaterials (Variables|/Game/Blueprints/BP_ModulePiece.BP_ModulePiece_C|GetCube _asbp_module_piece) "HueShift" (Variables|Default|GetRandomHueShift))
    (Rendering|Material|SetScalarParameterValueonMaterials (Variables|/Game/Blueprints/BP_ModulePiece.BP_ModulePiece_C|GetCube _asbp_module_piece) "Desaturate" (Variables|Default|GetRandomSaturationShift))))

(event Custom|ModuleUsed
  (Variables|Default|SetUsed true)
  (for _array_element (Actor|GetAllChildActors true)
    (bind _asbp_module_piece (Utilities|Casting|CastToBP_ModulePiece _array_element))
    (Rendering|Material|SetMaterial (Variables|/Game/Blueprints/BP_ModulePiece.BP_ModulePiece_C|GetCube _asbp_module_piece) 0 "/Game/Material/M_Locked_Inst.M_Locked_Inst")
    (Rendering|Material|SetScalarParameterValueonMaterials (Variables|/Game/Blueprints/BP_ModulePiece.BP_ModulePiece_C|GetCube _asbp_module_piece) "HueShift" (Variables|Default|GetRandomHueShift))
    (Rendering|Material|SetScalarParameterValueonMaterials (Variables|/Game/Blueprints/BP_ModulePiece.BP_ModulePiece_C|GetCube _asbp_module_piece) "Desaturate" (Variables|Default|GetRandomSaturationShift))
    (Rendering|Material|SetVectorParameterValueonMaterials (Variables|/Game/Blueprints/BP_ModulePiece.BP_ModulePiece_C|GetCube _asbp_module_piece) "SubtractColour" (Math|Vector|MakeVector 1.0 1.0 1.0)))
  (Rendering|Components|TextRender|SetTextRenderColor (Variables|Default|GetTextRender) (Math|Color|MakeColor 255 255 255 255)))

(event Custom|RefreshModule
  (Variables|Default|SetUsed false)
  (for _array_element (Actor|GetAllChildActors true)
    (bind _asbp_module_piece (Utilities|Casting|CastToBP_ModulePiece _array_element))
    (Rendering|Material|SetMaterial (Variables|/Game/Blueprints/BP_ModulePiece.BP_ModulePiece_C|GetCube _asbp_module_piece) 0 "/Game/Material/M_Locked_Inst.M_Locked_Inst")
    (Rendering|Material|SetScalarParameterValueonMaterials (Variables|/Game/Blueprints/BP_ModulePiece.BP_ModulePiece_C|GetCube _asbp_module_piece) "HueShift" (Variables|Default|GetRandomHueShift))
    (Rendering|Material|SetScalarParameterValueonMaterials (Variables|/Game/Blueprints/BP_ModulePiece.BP_ModulePiece_C|GetCube _asbp_module_piece) "Desaturate" (Variables|Default|GetRandomSaturationShift))
    (Rendering|Material|SetVectorParameterValueonMaterials (Variables|/Game/Blueprints/BP_ModulePiece.BP_ModulePiece_C|GetCube _asbp_module_piece) "SubtractColour" (Math|Vector|MakeVector 0.0 0.0 0.0)))
  (Rendering|Components|TextRender|SetTextRenderColor (Variables|Default|GetTextRender) (Math|Color|MakeColor 0 0 0)))

(event EventBeginPlay
  (bind _outactors (Actor|GetAllActorsOfClass "/Game/Blueprints/BP_Brain.BP_Brain_C"))
  (Variables|Default|SetBP_Brain (Utilities|Array|Get(acopy) _outactors))
  (Variables|Default|SetStartPosition (Transformation|GetActorLocation))
  (Variables|Default|SetRandomHueShift (Math|Random|RandomFloatinRange 0.0 1.0))
  (Variables|Default|SetRandomSaturationShift (* (Math|Random|RandomFloatinRange 0.0 4.0) 2.0))
  (CallFunction|ColourChange))

(event Collision|EventActorBeginOverlap
  (params (OtherActor :type Actor%20Object%20Reference)))

(event EventTick
  (params (DeltaSeconds :type Float%20%28single-precision%29)))

(fn ConstructionScript
  (bind _axislength (Variables|Default|GetAxisLength))
  (bind _patterns (Variables|Default|GetPatterns))
  (bind _textrender (Variables|Default|GetTextRender))
  (bind _cubedistance (Variables|Default|GetCubeDistance))
  (bind _subpattern (Variables|Default|GetSubPattern))
  (bind _textrender_2 (Variables|Default|GetTextRender))
  (bind _axislength_2 (Variables|Default|GetAxisLength))
  (bind _subpattern_2 (Variables|Default|GetSubPattern))
  (bind _textrender_3 (Variables|Default|GetTextRender))
  (bind _cubedistance_2 (Variables|Default|GetCubeDistance))
  (bind _patterns_2 (Variables|Default|GetPatterns))
  (bind _returnvalue (Math|Conversions|ToFloat(Integer) _axislength_2))
  (bind _returnvalue_2 (/ _returnvalue 2.0))
  (bind _returnvalue_3 (* _cubedistance _returnvalue_2))
  (for (_array_element _array_index) (Variables|Default|GetShape)
    (if (== _array_element 1)
      (Utilities|Array|SetArrayElem _patterns (Math|Integer|%(Integer) _array_index _axislength) (+ (Utilities|Array|Get(acopy) _patterns (Math|Integer|%(Integer) _array_index _axislength)) 1))
      (Utilities|Array|SetArrayElem _patterns_2 (+ (/ _array_index _axislength) 3) (+ (Utilities|Array|Get(acopy) _patterns_2 (+ (/ _array_index _axislength) 3)) 1))
      (bind _returnvalue_4 (AddComponent|AddChildActorComponent false (Math|Transform|MakeTransform (- (Math|Vector|MakeVector _returnvalue_3 _returnvalue_3 0.0) (Math|Vector|MakeVector (* (Math|Conversions|ToFloat(Integer) (Math|Integer|%(Integer) _array_index _axislength)) _cubedistance_2) (* (Math|Conversions|ToFloat(Integer) (/ _array_index _axislength)) _cubedistance_2) 0.0)))))
      (ChildActorComponent|SetChildActorClass _returnvalue_4 "/Game/Blueprints/BP_ModulePiece.BP_ModulePiece_C")
      (Utilities|Array|Add (Variables|Default|GetPieces) (.AsBP%20Module%20Piece (Utilities|Casting|CastToBP_ModulePiece (Variables|/Script/Engine.ChildActorComponent|GetChildActor _returnvalue_4))))))
  (Rendering|Components|TextRender|SetText (Variables|Default|GetTextRender) (Utilities|Text|ToText(String) (Variables|Default|GetModuleString)))
  (for (_array_element_2 _array_index_2) (Variables|Default|GetPatterns)
    (if (>= _array_index_2 3)
      (if (>= _array_element_2 (Variables|Default|GetHighestPattern))
        (Variables|Default|SetHighestPattern _array_element_2)
        (Variables|Default|SetChosenPattern _array_index_2))
      (elif (> _array_element_2 (Variables|Default|GetHighestPattern))
        (Variables|Default|SetHighestPattern _array_element_2)
        (Variables|Default|SetChosenPattern _array_index_2))))
  (if (>= (Variables|Default|GetChosenPattern) 3)
    (Transformation|SetRelativeLocation _textrender (+ (* (Math|Vector|MakeVector 0.0 (* (- (Variables|Default|GetChosenPattern) 4) (Variables|Default|GetCubeDistance)) 0.0) -1.0) "128.000000,128.000000,200.000000") false false)
    (if (< (Variables|Default|GetHighestPattern) 3)
      (for (_array_element_3 _array_index_3) (Variables|Default|GetShape)
        (if (== _array_element_3 1)
          (Utilities|Array|SetArrayElem _subpattern_2 (Math|Integer|%(Integer) _array_index_3 3) (+ (Utilities|Array|Get(acopy) _subpattern_2 (Math|Integer|%(Integer) _array_index_3 3)) 1))))
      (for (_array_element_4 _array_index_4) (Variables|Default|GetSubPattern)
        (if (>= _array_element_4 2)
          (Variables|Default|SetHighestSubIndex (+ (Variables|Default|GetHighestSubIndex) _array_index_4))))
      (Transformation|SetRelativeLocation _textrender_3 (+ (Variables|/Script/Engine.SceneComponent|GetRelativeLocation _textrender_3) (* (Math|Vector|MakeVector (* (Variables|Default|GetCubeDistance) (- (Math|Conversions|ToFloat(Integer) (Variables|Default|GetHighestSubIndex)) 2.0)) 0.0 0.0) -0.5)) false false))
    (else
      (Transformation|SetRelativeRotation _textrender "-270.000000,-45.000000,-270.000000" false false)
      (Transformation|SetRelativeLocation _textrender (+ (* (Math|Vector|MakeVector (* (- (Variables|Default|GetChosenPattern) 1) (Variables|Default|GetCubeDistance)) 0.0 0.0) -1.0) "128.000000,128.000000,200.000000") false false)
      (if (< (Variables|Default|GetHighestPattern) 3)
        (Development|PrintString "I am stubby")
        (for (_array_element_5 _array_index_5) (Variables|Default|GetShape)
          (if (== _array_element_5 1)
            (Utilities|Array|SetArrayElem _subpattern (/ _array_index_5 3) (+ (Utilities|Array|Get(acopy) _subpattern (/ _array_index_5 3)) 1))))
        (for (_array_element_6 _array_index_6) (Variables|Default|GetSubPattern)
          (if (>= _array_element_6 (Variables|Default|GetHighestSub))
            (Variables|Default|SetHighestSub _array_element_6)
            (Variables|Default|SetHighestSubIndex _array_index_6)))
        (Transformation|SetRelativeLocation _textrender_2 (+ (Variables|/Script/Engine.SceneComponent|GetRelativeLocation _textrender_2) (* (Math|Vector|MakeVector 0.0 (* (+ (* (* (Variables|Default|GetHighestSubIndex) 2) -1) 1) (Variables|Default|GetCubeDistance)) 0.0) 0.5)) false false)
        (Development|PrintString (Utilities|String|ToString(Vector) (* (Math|Vector|MakeVector 0.0 (* (+ (* (* (Variables|Default|GetHighestSubIndex) 2) -1) 1) (Variables|Default|GetCubeDistance)) 0.0) 0.5)) true true "(R=0.000000,G=0.660000,B=1.000000,A=1.000000)" 4.0)))))