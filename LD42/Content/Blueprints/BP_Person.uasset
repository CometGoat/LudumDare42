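; BP_Person is a character built from textured body, arm and head parts, animated procedurally by rotating anchor components.
; The construction script uses AppearanceSwitch to choose clothing and shape textures on dynamic materials for body and arms.
; Timelines drive Idle and Talk pitch swings, with AppearanceSwitch varying the Talk motion.
; BeginPlay runs Idle, then ReturnToStart eases rotations to zero before Talk; StoreStartPoints is an empty stub.
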(event Custom|Talk
  (bind _appearanceswitch (Variables|Default|GetAppearanceSwitch))
  (bind _newtrack_0 (Timeline|IdleAnim PlayFromStart)
    (:Update
      (Transformation|SetRelativeRotation (Variables|Default|GetAnchor_Body) (Math|Rotator|MakeRotator 0.0 (/ _newtrack_0 2.0) 0.0) false false)
      (Transformation|SetRelativeRotation (Variables|Default|GetAnchor_Arm) (Math|Rotator|MakeRotator 0.0 (select _appearanceswitch (* _newtrack_0 -1.0) _newtrack_0) 0.0) false false)
      (Transformation|SetRelativeRotation (Variables|Default|GetAnchor_Arm_Left) (Math|Rotator|MakeRotator 0.0 (select _appearanceswitch (* _newtrack_0 -1.0) _newtrack_0) 0.0) false false)
      (Transformation|SetRelativeRotation (Variables|Default|GetAnchor_Head) (Math|Rotator|MakeRotator 0.0 (select _appearanceswitch (* (* (Math|Float|Sqrt _newtrack_0) 4.0) -1.0) (* (Math|Float|Sqrt _newtrack_0) 8.0)) 0.0) false false))))

(event Custom|ReturnToStart
  (CallFunction|StopAnims)
  (bind _newtrack_0 (Timeline|Return PlayFromStart)
    (:Update
      (for _array_element (Utilities|Array|MakeArray (Variables|Default|GetAnchor_Body) (Variables|Default|GetAnchor_Arm) (Variables|Default|GetAnchor_Arm_Left) (Variables|Default|GetAnchor_Head))
        (Transformation|SetRelativeRotation _array_element (Math|Rotator|Lerp(Rotator) (Variables|/Script/Engine.SceneComponent|GetRelativeRotation _array_element) "0, 0, 0" _newtrack_0) false false)))))

(event Custom|StoreStartPoints)

(event Custom|StopAnims
  (bind _appearanceswitch (Variables|Default|GetAppearanceSwitch))
  (Utilities|FlowControl|Sequence
    (:then_0
      (bind _newtrack_0 (Timeline|IdleAnim Stop)
        (:Update
          (Transformation|SetRelativeRotation (Variables|Default|GetAnchor_Body) (Math|Rotator|MakeRotator 0.0 (/ _newtrack_0 2.0) 0.0) false false)
          (Transformation|SetRelativeRotation (Variables|Default|GetAnchor_Arm) (Math|Rotator|MakeRotator 0.0 (select _appearanceswitch (* _newtrack_0 -1.0) _newtrack_0) 0.0) false false)
          (Transformation|SetRelativeRotation (Variables|Default|GetAnchor_Arm_Left) (Math|Rotator|MakeRotator 0.0 (select _appearanceswitch (* _newtrack_0 -1.0) _newtrack_0) 0.0) false false)
          (Transformation|SetRelativeRotation (Variables|Default|GetAnchor_Head) (Math|Rotator|MakeRotator 0.0 (select _appearanceswitch (* (* (Math|Float|Sqrt _newtrack_0) 4.0) -1.0) (* (Math|Float|Sqrt _newtrack_0) 8.0)) 0.0) false false))))
    (:then_1
      (bind _newtrack_0_2 (Timeline|IdleAnim_True Stop)
        (:Update
          (Transformation|SetRelativeRotation (Variables|Default|GetAnchor_Body) (Math|Rotator|MakeRotator 0.0 (/ _newtrack_0_2 2.0) 0.0) false false)
          (Transformation|SetRelativeRotation (Variables|Default|GetAnchor_Arm) (Math|Rotator|MakeRotator 0.0 (* _newtrack_0_2 -0.5) 0.0) false false)
          (Transformation|SetRelativeRotation (Variables|Default|GetAnchor_Arm_Left) (Math|Rotator|MakeRotator 0.0 (* _newtrack_0_2 -0.5) 0.0) false false))))))

(event Custom|Idle
  (bind _newtrack_0 (Timeline|IdleAnim_True PlayFromStart)
    (:Update
      (Transformation|SetRelativeRotation (Variables|Default|GetAnchor_Body) (Math|Rotator|MakeRotator 0.0 (/ _newtrack_0 2.0) 0.0) false false)
      (Transformation|SetRelativeRotation (Variables|Default|GetAnchor_Arm) (Math|Rotator|MakeRotator 0.0 (* _newtrack_0 -0.5) 0.0) false false)
      (Transformation|SetRelativeRotation (Variables|Default|GetAnchor_Arm_Left) (Math|Rotator|MakeRotator 0.0 (* _newtrack_0 -0.5) 0.0) false false))))

(event EventBeginPlay
  (CallFunction|Idle)
  (CallFunction|StoreStartPoints)
  (Utilities|FlowControl|Delay 7.0)
  (CallFunction|ReturntoStart)
  (Utilities|FlowControl|Delay 1.0)
  (CallFunction|Talk))

(event Collision|EventActorBeginOverlap
  (params (OtherActor :type Actor%20Object%20Reference)))

(event EventTick
  (params (DeltaSeconds :type Float%20%28single-precision%29)))

(fn ConstructionScript
  (bind _body (Variables|Default|GetBody))
  (bind _arm (Variables|Default|GetArm))
  (bind _arm_left (Variables|Default|GetArm_Left))
  (bind _appearanceswitch (Variables|Default|GetAppearanceSwitch))
  (bind _returnvalue (Rendering|Material|CreateDynamicMaterialInstance _body 0 (Rendering|Material|GetMaterial _body 0) "None" :!class /Script/Engine.PrimitiveComponent))
  (Rendering|Material|SetTextureParameterValue _returnvalue "ClothesTexture" (select (Variables|Default|GetAppearanceSwitch) "/Game/Textures/FloralPrint_2.FloralPrint_2" "/Game/Textures/Plaid_Square.Plaid_Square"))
  (Rendering|Material|SetTextureParameterValue _returnvalue "BodyTexture" (select _appearanceswitch "/Game/Textures/WomanShirtPose.WomanShirtPose" "/Game/Textures/Body_Alpha.Body_Alpha"))
  (Transformation|SetRelativeScale3D (Variables|Default|GetBody) (select _appearanceswitch "1.000000,1.000000,1.000000" "1.000000,1.000000,1.000000"))
  (bind _returnvalue_2 (Rendering|Material|CreateDynamicMaterialInstance _arm 0 (Rendering|Material|GetMaterial _arm 0) "None" :!class /Script/Engine.PrimitiveComponent))
  (Rendering|Material|SetTextureParameterValue _returnvalue_2 "ClothesTexture" "/Game/Textures/Skin.Skin")
  (Rendering|Material|SetTextureParameterValue _returnvalue_2 "BodyTexture" (select (Variables|Default|GetAppearanceSwitch) "/Game/Textures/ArmFemale_Alpha.ArmFemale_Alpha" "/Game/Textures/Arm_alpha.Arm_alpha"))
  (bind _returnvalue_3 (Rendering|Material|CreateDynamicMaterialInstance _arm_left 0 (Rendering|Material|GetMaterial _arm_left 0) "None" :!class /Script/Engine.PrimitiveComponent))
  (Rendering|Material|SetTextureParameterValue _returnvalue_3 "ClothesTexture" "/Game/Textures/Skin.Skin")
  (Rendering|Material|SetTextureParameterValue _returnvalue_3 "BodyTexture" (select (Variables|Default|GetAppearanceSwitch) "/Game/Textures/ArmFemale_Alpha.ArmFemale_Alpha" "/Game/Textures/Arm_alpha.Arm_alpha")))