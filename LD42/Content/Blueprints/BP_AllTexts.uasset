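; Narrative text actor that plays the story outcome of a mission, currently only a supermarket food-shopping task, based on the player's installed brain modules.
; LoadReferences caches BP_Brain's installed modules and the player controller's text box.
; NextSection picks the installed module with the lowest grade number for the event as SelectedOutcome.
; Mission1_1 uses that index to select three hardcoded passages, polling TextFinished on short delays to type them in sequence.
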(event Custom|NextSection
  (params (Mission :type Integer) (Event :type Integer))
  (bind _mission_1_1 (Variables|Default|GetMission_1_1))
  (bind _output (Utilities|Array|Get(acopy) _mission_1_1 Event))
  (Variables|Default|SetHighestGrade 999)
  (switch int Mission
    (:0
      (for _array_element (Variables|Default|GetLoadedModules)
        (if (and (Utilities|Array|ContainsItem (.modules _output) _array_element) (< (Utilities|Array|Get(acopy) (.grades _output) (Utilities|Array|FindItem (.modules _output) _array_element)) (Variables|Default|GetHighestGrade)))
          (Variables|Default|SetHighestGrade (Utilities|Array|Get(acopy) (.grades _output) (Utilities|Array|FindItem (.modules _output) _array_element)))
          (bind _output_get (Variables|Default|SetSelectedOutcome (Utilities|Array|FindItem (.modules _output) _array_element)))
          (Development|PrintString (Utilities|String|Append "Loaded module: " (Utilities|String|ToString(Integer) _output_get)))))
      (CallFunction|Mission11))))

(event Custom|LoadReferences
  (bind _outactors (Actor|GetAllActorsOfClass "/Game/Blueprints/BP_Brain.BP_Brain_C"))
  (Variables|Default|SetLoadedModules (Variables|/Game/Blueprints/BP_Brain.BP_Brain_C|GetInstalledModules (Utilities|Array|Get(acopy) _outactors)))
  (Variables|Default|SetW_TextBox (Variables|/Game/Game/BP_PlayerController.BP_PlayerController_C|GetW_TextBox (.AsBP%20Player%20Controller (Utilities|Casting|CastToBP_PlayerController (Game|GetPlayerController 0))))))

(event Custom|Mission1_1
  (bind _w_textbox (Variables|Default|GetW_TextBox))
  (bind _w_textbox_2 (Variables|Default|GetW_TextBox))
  (bind _w_textbox_3 (Variables|Default|GetW_TextBox))
  (Development|PrintString "Playing mission 1_1")
  (if (Variables|/Game/UI/Widgets/W_TextBox.W_TextBox_C|GetTextFinished _w_textbox_2) :!label _label
    (Variables|/Game/UI/Widgets/W_TextBox.W_TextBox_C|SetTextFinished _w_textbox_2 false)
    (Default|LoopThroughCharacters _w_textbox_2 (Utilities|Select :Index (Variables|Default|GetSelectedOutcome) :Option%200 (Utilities|String|MakeLiteralString "You walk into the TESCO PLC. There’s an overwhelming amount of things inside: packets of potatoes shaped as human faces, and cans of corn with rugged green giants on the front, for example.") :Option%201 (Utilities|String|MakeLiteralString "You walk into the TESCO PLC. There’s an overwhelming amount of things inside: packets of potatoes shaped as human faces, and cans of corn with rugged green giants on the front, for example. All of them look like they can be deep fried.") :Option%202 "You walk into the TESCO PLC. There’s an overwhelming amount of things inside: tubes of sprinkles called 100s and 1000s (even though they contain an average of 10,832 sprinkles per tube on average), and cans of corn with rugged green giants on the front, for example." :Option%203 "You walk into the TESCO PLC. There’s an overwhelming amount of things inside: small salty squares called ‘OXO cubes’, and small spiky grey things that are either artichokes or armadillos, for example. " :Option%204 "You walk into the TESCO PLC. There’s an overwhelming amount of things inside: packets of potatoes shaped as human faces, and cans of corn with rugged green giants on the front, for example." :Option%205 "You walk into the TESCO PLC. There’s an overwhelming amount of things inside: packets of potatoes shaped as human faces, and cans of corn with rugged green giants on the front, for example." :Option%206 "You walk into the TESCO PLC. There’s an overwhelming amount of things inside: packets of potatoes shaped as human faces, and cans of corn with rugged green giants on the front, for example." :Option%207 "You walk into the TESCO PLC. There’s an overwhelming amount of things inside: bottled cow secretion, and crackers belonging to someone called Jacob, for example." :Option%208 "You walk into the TESCO PLC. There’s an overwhelming amount of things inside: packs of tiny spears called ‘toothpicks’, and chocolate Kit Kat bars imploring you to ‘take a break’, for example." :Option%209 "You walk into the TESCO PLC. There’s an overwhelming amount of things inside: packs of tiny spears called ‘toothpicks’, and chocolate Kit Kat bars imploring you to ‘take a break’, for example." :Option%2010 "You walk into the TESCO PLC. There’s an overwhelming amount of things inside: bottled cow secretion, and crackers belonging to someone called Jacob, for example." :Option%2011 "You walk into the TESCO PLC. There’s an overwhelming amount of things inside: small salty squares called ‘OXO cubes’, and small spiky grey things that are either artichokes or armadillos, for example." :Option%2012 "You walk into the TESCO PLC. There’s an overwhelming amount of things inside: small salty squares called ‘OXO cubes’, and so, so, so many rows of bananas, for example." :Option%2013 "You walk into the TESCO PLC. There’s an overwhelming amount of things inside: small salty squares called ‘OXO cubes’, and so, so, so many rows of bananas, for example."))
    (Utilities|FlowControl|Delay 0.2 :!label _label_2)
    (if (Variables|/Game/UI/Widgets/W_TextBox.W_TextBox_C|GetTextFinished _w_textbox_2)
      (Variables|/Game/UI/Widgets/W_TextBox.W_TextBox_C|SetTextFinished _w_textbox false)
      (Default|LoopThroughCharacters _w_textbox (Utilities|Select :Index (Variables|Default|GetSelectedOutcome) :Option%200 (Utilities|String|MakeLiteralString "Spaghetti module…loading…loaded! 
Insight: Spaghetti is a wheat-based material that is popular with humans. 
 
Eventually you find the section with spaghetti in it. There is a lot of it: 
-        long thin spaghettis 
-        long fat spaghettis 
-        tiny squiggle spaghettis 
-        cute bow-tie spaghettis 
 
You watch another human pick up a packet of the cute bow-tie spaghettis, so you do this too. On the back of the packet, a tiny chef recommends you cook this with ‘pesto’. You pick up a jar and put it in your metal bag.") :Option%201 (Utilities|String|MakeLiteralString "Deep Fry module…loading…loaded! 
Insight: Humans will often put their food under duress before eating it. 
 
‘If I want to deep fry, what do you suggest?’ you ask one human. 
‘…’ they say. 
Then, they say ‘you need…oil? And a thing to fry?’") :Option%202 "Potato module…loading…loaded! 
Insight: Potatoes can be boiled or mashed or stuck in a stew. 
 
Eventually you find the section with potatoes.  
You get some labelled ‘for boiling’ and some ‘for mashing’ to be safe. There appear to be no potatoes ‘for stewing’." :Option%203 "Canned food module…loading…loaded!  
Insight: If the apocalypse comes, food in cans will be the king of all foods. 
 
Eventually you find the section full of canned foods. And oh boy, are there a lot. There are: 
-        Cans of corn, with a dashing green giant on the front 
-        Cans of squished up fish 
-        Cans of beans in orange sauce 
-        Cans of chicken soup that provides nutrients for the soul" :Option%204 "Weather module…loading…loaded! 
Insight: The sky does whatever it wants. Humans love to talk about it. 
 
You try to engage a human for help. 
‘How about…this…weather?’ you ask. You gesture at the ceiling. 
‘…’ says the human. Then they say ‘Uh huh,’ and walk away. 
‘Wait! But…the sunshine!’ you shout.  
They're now pushing their metal box away at maximum speed." :Option%205 "Gardening module…loading…loaded! 
Insight: Humans will sometimes nurture plants using water, sunlight, and soil. 
 
‘How do I grow some food materials?’ you ask.  
‘Just buy some bloody pasta,’ the human says.  
‘How do you grow a pasta?’ you ask.  
But they’re already pushing their metal box away at maximum speed." :Option%206 "Slam Poetry module…loading…loaded! 
Insight: Slam Poetry is word vomit…but good. 
 
You try to engage a human through the power of slam poetry. 
‘I stand here amongst these aisles, surrounded by sigils of consumerism, starved of true choice, drowning in corporate mockery.’ you say. 
‘Mate… what the hell,’ the human says.  
You slam the human with your final line: ‘CORPORATE MOCKERY’.  
They’re now pushing their metal box away at maximum speed." :Option%207 "Coffee Art module…loading…loaded!  
Insight: A craft passed down from barista to barista. Often takes the form of a heart, a flower, or sometimes a penis. 
 
You try to engage a human for help. 
‘Do you know the craft of coffee art?’ you ask.  
‘Bruh.’ the human says.  
‘You’re a…coffee bruh?’ you ask.  
They roll their eyes. 
‘Coffee’s down that way,’ they say." :Option%208 "Mould module…loading…loaded! 
Insight: Mould is fuzzy, but humans hate it. It should not be on food. 
 
‘I want to know about the mould prevalence in your food items,’ you ask a human with a TESCO PLC shirt. 
The human looks worried. 
‘Did you purchase a mouldy item? We can sort that out for you,’ they say. 
‘No. I want to know about the mould prevalence here,’ you explain patiently. 
‘…’ the human says. Then they say ‘the blue cheese is in aisle 5’. " :Option%209 "Machete module…loading…loaded! 
Insight: Machetes are sharp. And stabby! 
 
You try to engage a human for help. 
‘Don’t you love how sharp machetes are?’ you ask.  
‘Are you th-threatening me?’ the human says. They are shaking. 
‘I just want to chat about machetes’ you say.  
But they’re already pushing their metal box away at maximum speed." :Option%2010 "Parents module…loading…loaded!  
Insight: An adult-sized human who has somehow come to be responsible for a child-sized human. 
 
You try to engage a human for help. 
‘Do you know where my parents are?’ you ask.  
‘Oh. Are you…lost?’ the human says.  
‘I’m just looking for some parents’ you say.  
They nod urgently. They take your hand! 
‘Okay, come with me,’ they say." :Option%2011 "Tattoos module…loading…loaded!  
Insight: An ink-based decoration that can go almost anywhere on the human body… Yes, even there. 
 
You try to engage a human for help. 
‘Let’s get matching tattoos!’ you say.  
‘…’ the human says. Then they slowly turn around and wheel their metal box away, occasionally turning around to eye you suspiciously. 
You’re left alone, with no food and no tattoo buddy." :Option%2012 "Teeth module…loading…loaded!  
Insight: Found inside the mouth, they are useful for mashing food and biting other humans. 
 
You look for things that are good for sinking your teeth into. It turns out there are a lot: 
-        A square piece of rubbery cheese  
-        A cucumber 
-        A raw steak 
-        A wibbly wobbly jelly" :Option%2013 "Rocks module…loading…loaded!  
Insight: A very versatile material. Can be used as paper weights, pets, or genre of music. 
 
You try to engage a human for help. 
‘So, rocks huh?’ you say.  
‘…’ the human says. They slowly turn around and wheel their metal box away, occasionally turning around to eye you suspiciously. 
‘Can’t we talk about rocks for a minute, though?’ you shout. 
They’re now pushing their metal box away at maximum speed."))
      (Utilities|FlowControl|Delay 0.2 :!label _label_3)
      (if (Variables|/Game/UI/Widgets/W_TextBox.W_TextBox_C|GetTextFinished _w_textbox_2)
        (Variables|/Game/UI/Widgets/W_TextBox.W_TextBox_C|SetTextFinished _w_textbox_3 false)
        (Default|LoopThroughCharacters _w_textbox_3 (Utilities|Select :Index (Variables|Default|GetSelectedOutcome) :Option%200 (Utilities|String|MakeLiteralString "You have now obtained a jar of pureed geese faeces and bow ties! 
First task complete! 
Proceed…") :Option%201 (Utilities|String|MakeLiteralString "So you buy 10 litres of oil and a can of the corn with a rugged green giant on the front. 
 
You have now obtained a lot of oil and a can of corn! 
First task complete! 
Proceed…") :Option%202 "You have now obtained many, many potatoes! 
First task complete! 
Proceed…" :Option%203 "You decide to get one of each, in order to sample the true range of human cuisine. 
 
You have obtained many canned goods! 
First task complete! Proceed…" :Option%204 "First task failed. 
Re-evaluate module choices…" :Option%205 "Eventually you acquire some ready-grown pasta in a bag. You cannot find any blood. This will have to do. 
 
You have obtained a bag of ready-grown pasta! 
First task complete! 
Proceed…" :Option%206 "First task failed. 
Re-evaluate module choices…" :Option%207 "You follow their pointing, and sure enough there is an aisles full of all sorts of coffee-based goods. Even though coffee is liquid, the coffee products here are all solid. Perhaps they can be used as food? You take a few different kinds of grounds to be safe.  
 
 
You have obtained so many ground bits of coffee! 
First task complete!  
Proceed…" :Option%208 "The human is correct; there is one food here that is being mouldy on purpose, and it is a cheese in aisle 5. 
 
You have obtained a smelly hunk of blue cheese! 
First task complete! 
Proceed…" :Option%209 "First task failed. 
Re-evaluate module choices…" :Option%2010 "You end up sat with a human wearing a TESCO PLC shirt, whilst a speaker politely requests your parents come and pick you up. Since your parents are on the other side of the galaxy, they don’t turn up. 
 
First task failed. 
Re-evaluate module choices…" :Option%2011 "First task failed. 
Re-evaluate module choices…" :Option%2012 "You take one of each for good measure. 
 
You have obtained various chewable items! 
First task complete!  
Proceed…" :Option%2013 "First task failed. 
Re-evaluate module choices…"))
        (else
          (goto _label_3)))
      (else
        (goto _label_2)))
    (else
      (Utilities|FlowControl|Delay 0.2)
      (goto _label))))

(event EventBeginPlay)

(event Collision|EventActorBeginOverlap
  (params (OtherActor :type Actor%20Object%20Reference)))

(event EventTick
  (params (DeltaSeconds :type Float%20%28single-precision%29)))

(fn ConstructionScript)