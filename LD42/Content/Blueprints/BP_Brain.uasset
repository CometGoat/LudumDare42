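; BP_Brain builds a flat grid of BP_Tile child actors, AxisX by AxisY in count, and stores them in Tiles.
; The construction script spaces tiles by CubeDistance, offset by half the grid size, deriving positions from the flat index.
; ResizeBrain destroys all child actors and rebuilds the grid at runtime.
; Y uses index / AxisY rather than AxisX, except ResizeBrain switches to index % AxisY for non-square sizes.
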(event Custom|ResizeBrain
  (bind _axis_y (Variables|Default|GetAxis_Y))
  (bind _cubedistance (Variables|Default|GetCubeDistance))
  (bind _axis_x (Variables|Default|GetAxis_X))
  (Utilities|Array|Clear (Variables|Default|GetTiles))
  (for _array_element (Actor|GetAllChildActors true)
    (Actor|DestroyActor _array_element))
  (Utilities|Array|Resize (Variables|Default|GetGrid) (* (Variables|Default|GetAxis_X) (Variables|Default|GetAxis_Y)))
  (for (_ _array_index) (Variables|Default|GetGrid)
    (bind _returnvalue (AddComponent|AddChildActorComponent false (Math|Transform|MakeTransform (- (Math|Vector|MakeVector (* (Math|Conversions|ToFloat(Integer) (Math|Integer|%(Integer) _array_index _axis_x)) _cubedistance) (* (Math|Conversions|ToFloat(Integer) (select (== _axis_x _axis_y) (/ _array_index _axis_y) (Math|Integer|%(Integer) _array_index _axis_y))) _cubedistance) 0.0) (* (Math|Vector|MakeVector (/ (Math|Conversions|ToFloat(Integer) (Variables|Default|GetAxis_X)) 2.0) (/ (Math|Conversions|ToFloat(Integer) (Variables|Default|GetAxis_Y)) 2.0) 0.0) (Variables|Default|GetCubeDistance))))))
    (Utilities|Array|Add (Variables|Default|GetTiles) (.AsBP%20Tile (Utilities|Casting|CastToBP_Tile (Variables|/Script/Engine.ChildActorComponent|GetChildActor _returnvalue))))))

(event EventBeginPlay)

(event Collision|EventActorBeginOverlap
  (params (OtherActor :type Actor%20Object%20Reference)))

(event EventTick
  (params (DeltaSeconds :type Float%20%28single-precision%29)))

(fn ConstructionScript
  (bind _cubedistance (Variables|Default|GetCubeDistance))
  (Utilities|Array|Resize (Variables|Default|GetGrid) (* (Variables|Default|GetAxis_X) (Variables|Default|GetAxis_Y)))
  (for (_ _array_index) (Variables|Default|GetGrid)
    (bind _returnvalue (AddComponent|AddChildActorComponent false (Math|Transform|MakeTransform (- (Math|Vector|MakeVector (* (Math|Conversions|ToFloat(Integer) (Math|Integer|%(Integer) _array_index (Variables|Default|GetAxis_X))) _cubedistance) (* (Math|Conversions|ToFloat(Integer) (/ _array_index (Variables|Default|GetAxis_Y))) _cubedistance) 0.0) (* (Math|Vector|MakeVector (/ (Math|Conversions|ToFloat(Integer) (Variables|Default|GetAxis_X)) 2.0) (/ (Math|Conversions|ToFloat(Integer) (Variables|Default|GetAxis_Y)) 2.0) 0.0) (Variables|Default|GetCubeDistance))))))
    (Utilities|Array|Add (Variables|Default|GetTiles) (.AsBP%20Tile (Utilities|Casting|CastToBP_Tile (Variables|/Script/Engine.ChildActorComponent|GetChildActor _returnvalue))))))